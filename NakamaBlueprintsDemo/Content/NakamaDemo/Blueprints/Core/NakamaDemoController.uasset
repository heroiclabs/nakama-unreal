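; Player controller for the Nakama demo that creates the main UI and a default Nakama client on BeginPlay.
; After authentication it stores the session, connects a realtime client and binds matchmaking, chat, presence, notification, party ticket, disconnect and error listeners.
; Those listeners mostly raise on-screen notifications, skipping the user's own chat and presence.
; Other events relay errors, matches, tickets, private messages, groups and account changes to the main widget.
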(event Custom|MatchmakerMatched
  (params (Match :type Nakama%20Matchmaker%20Matched%20Structure%20%28by%20ref%29))
  ;[1 1 1] Show Popup when a Match has been found
  (Default|RemoveMatchmakerTicket (Variables|Default|GetMainUI) (.Ticket (Utilities|Struct|BreakNakamaMatchmakerMatched Match)))
  (CallFunction|ShowNotification "Matched!" "NewEnumerator4")
  (Default|ShowMatchmakerMatched (Variables|Default|GetMainUI) Match))

(event Custom|OnChatMessage
  (params (ChannelMessage :type Nakama%20Channel%20Message%20Structure%20%28by%20ref%29))
  (bind (_channelid _messageid _code _senderid _username _content) (Utilities|Struct|BreakNakamaChannelMessage ChannelMessage))
  ;[1 1 1] Show chat message notification
  (if (not (Utilities|Enum|Equal(Enum) _senderid (.userid (Variables|/Script/NakamaUnreal.NakamaSession|GetSessionData (CallFunction|GetCurrentSession)))))
    (bind _returnvalue (Class|NakamaLibrary|ChatMessageJsontoStruct _content))
    (CallFunction|ShowNotification (Utilities|Text|FormatText "{Sender} : {Message}" _username (.ChatMessage (Utilities|Struct|BreakNakamaChatMessage _returnvalue))) "NewEnumerator2")))

(event Custom|OnStatusPresence
  (params (UserPresenceData :type Nakama%20Status%20Presence%20Event%20Structure%20%28by%20ref%29))
  (bind (_joins _leaves) (Utilities|Struct|BreakNakamaStatusPresenceEvent UserPresenceData))
  (bind _session (CallFunction|GetCurrentSession))
  (bind _sessiondata (Variables|/Script/NakamaUnreal.NakamaSession|GetSessionData _session))
  ;[1 1 1] Display Statuses
  (Utilities|FlowControl|Sequence
    (:then_0
      ;;[1 1 1] Status Joins
      (for _array_element _joins
        (if (Utilities|Enum|NotEqual(Enum) (.UserID (Utilities|Struct|BreakNakamaUserPresence _array_element)) (.userid _sessiondata))
          (CallFunction|ShowNotification (Utilities|Text|FormatText "Joins: {Username} : {Status}" (.Username (Utilities|Struct|BreakNakamaUserPresence _array_element)) (.Status (Utilities|Struct|BreakNakamaUserPresence _array_element))) "NewEnumerator2"))))
    (:then_1
      ;;[1 1 1] Status Joins
      (for _array_element_2 _leaves
        (if (Utilities|Enum|NotEqual(Enum) (.UserID (Utilities|Struct|BreakNakamaUserPresence _array_element_2)) (.userid _sessiondata))
          _)))))

(event Custom|OnNotification
  (params (NotificationData :type Nakama%20Notification%20List%20Structure%20%28by%20ref%29))
  ;[1 1 1] Display simple notifications, must be sent server-side or via RPCs
  (for _array_element (.Notifications (Utilities|Struct|BreakNakamaNotificationList NotificationData))
    (CallFunction|ShowNotification (Utilities|Text|FormatText "Notification: {Subject} : {Content}" (.Subject (Utilities|Struct|BreakNakamaNotification _array_element)) (.Content (Utilities|Struct|BreakNakamaNotification _array_element))) "NewEnumerator2")))

(event Custom|OnPartyMatchmakerTicket
  (params (Ticket :type Nakama%20Party%20Matchmaker%20Ticket%20Structure%20%28by%20ref%29))
  ;[1 1 1] Add Party Matchmaker Ticket (Not leader)
  (Default|AddMatchmakerTicket (Variables|/Game/NakamaDemo/Widgets/WBP_Main.WBP_Main_C|GetWBP_Matchmaking (Variables|Default|GetMainUI)) (.Ticket (Utilities|Struct|BreakNakamaPartyMatchmakerTicket Ticket)) "PARTY"))

(event Custom|OnDisconnect
  (params (DisconnectInfo :type Nakama%20Disconnect%20Info%20Structure%20%28by%20ref%29))
  (bind (_code _reason) (Utilities|Struct|BreakNakamaDisconnectInfo DisconnectInfo))
  ;[1 1 1] Disconnected Event
  (CallFunction|ShowNotification (Utilities|Text|FormatText "Disconnected: {Code} : {Reason}" _code _reason) "NewEnumerator1"))

(event Custom|OnErrorEvent
  (params (Error :type Nakama%20Rt%20Error%20Structure%20%28by%20ref%29))
  ;[1 1 1] Error Event
  (CallFunction|ShowNotification (Utilities|Text|ToText(String) (.Message (Utilities|Struct|BreakNakamaRtError Error))) "NewEnumerator1"))

(event EventShowNotification
  (params (Message :type Text) (Severity :type ENotificationSeverity%20Enum :default "NewEnumerator0"))
  ;[1 1 1] Show Notification
  (Default|ShowNotificationMessage (Variables|Default|GetMainUI) Message Severity))

(event EventBeginPlay
  ;[1 1 1] Create Default Widget and Setup Default Client in Subsystem
  (bind _returnvalue (UserInterface|CreateWidget "/Game/NakamaDemo/Widgets/WBP_Main.WBP_Main_C" self))
  (bind _output_get (Variables|Default|SetMainUI _returnvalue))
  (UserInterface|Viewport|AddtoViewport _output_get 0)
  (Input|SetInputModeGameandUI self 0 "DoNotLock" true false)
  (Variables|Default|SetbShowMouseCursor true)
  ;[0 1 0.06848] SETUP YOUR VALUES HERE
  (bind _returnvalue_2 (Class|NakamaClient|CreateDefaultClient "defaultkey" "127.0.0.1" 7350 false true)) ; If Enable Debug is set, it will enable console logging with debug level
  (Variables|Default|SetNakamaClient _returnvalue_2))

(event EventAccountChanged
  (params (Account :type Nakama%20Account%20Structure))
  ;[1 1 1] Account
  (Rendering|Components|TextRender|SetText (Variables|/Game/NakamaDemo/Widgets/WBP_Main.WBP_Main_C|GetWelcomeText (Variables|Default|GetMainUI)) (Utilities|Text|ToText(String) (.Username (Utilities|Struct|BreakNakamaUser (.user Account))))))

(event EventOpenPrivateMessage
  (params (UserId :type String))
  ;[1 1 1] Open Private Message Directly from Friend
  (Default|OpenPrivateMessage (Variables|Default|GetMainUI) UserId))

(event EventAddMatch
  (params (AddedMatch :type Nakama%20Match%20Structure))
  (bind _mainui (Variables|Default|GetMainUI))
  ;[1 1 1] Add Match to UI
  (Default|AddMatch (Variables|/Game/NakamaDemo/Widgets/WBP_Main.WBP_Main_C|GetWBP_Realtime _mainui) AddedMatch)
  (Default|ShowMatches _mainui))

(event EventAddTicket
  (params (TickedId :type String) (MapName :type String))
  ;[1 1 1] Add Ticket as Leader (local)
  (Default|AddMatchmakerTicket (Variables|/Game/NakamaDemo/Widgets/WBP_Main.WBP_Main_C|GetWBP_Matchmaking (Variables|Default|GetMainUI)) TickedId MapName))

(event EventRemoveTicket
  (params (TicketId :type String))
  ;[1 1 1] Remove Ticket from UI
  (Default|RemoveTicket (Variables|/Game/NakamaDemo/Widgets/WBP_Main.WBP_Main_C|GetWBP_Matchmaking (Variables|Default|GetMainUI)) TicketId))

(event EventRefreshUserGroups
  ;[1 1 1] Refresh Groups
  (Default|ListUserGroups (Variables|/Game/NakamaDemo/Widgets/WBP_Main.WBP_Main_C|GetWBP_Groups (Variables|Default|GetMainUI))))

(event EventOnAuthenticated
  (params (Session :type Nakama%20Session%20Object%20Reference))
  (bind _sessiondata (Variables|/Script/NakamaUnreal.NakamaSession|GetSessionData Session))
  (bind _username (Utilities|Struct|BreakNakamaUserSession _sessiondata))
  (bind _returnvalue (Utilities|String|Append "Authenticated as: " _username))
  ;[1 1 1] Post Authentication
  (Variables|Default|SetUserSession Session)
  (Variables|Default|SetCurrentSessionData _sessiondata) ; Store this locally for convenience
  (Development|PrintString _returnvalue true true "(R=0.000000,G=1.000000,B=0.176688,A=1.000000)")
  (CallFunction|ShowNotification (Utilities|Text|ToText(String) _returnvalue) "NewEnumerator4")
  (Rendering|Components|TextRender|SetText (Variables|/Game/NakamaDemo/Widgets/WBP_Main.WBP_Main_C|GetWelcomeText (Variables|Default|GetMainUI)) (Utilities|Text|ToText(String) _username))
  ;;[0 1 0.06848] SETUP YOUR VALUES HERE
  (bind _returnvalue_2 (Class|NakamaClient|SetupRealtimeClient (Variables|Default|GetNakamaClient)))
  (bind _output_get (Variables|Default|SetNakamaRealtimeClient _returnvalue_2))
  (|Connect _output_get (Variables|Default|GetUserSession) true
    (:OnError
      (Development|PrintString "Failed to Setup Realtime Client!" true true "(R=1.000000,G=0.000000,B=0.027472,A=1.000000)")
      (CallFunction|ShowNotification "Failed to Setup Realtime Client!" "NewEnumerator1"))
    (:OnSuccess
      (Development|PrintString "Realtime Client Setup Success!" true true "(R=0.000000,G=1.000000,B=0.075578,A=1.000000)")
      (CallFunction|ShowNotification "Realtime Client Setup Success!" "NewEnumerator4")
      (Class|NakamaRealtimeClient|SetListenerAllCallbacks (Variables|Default|GetNakamaRealtimeClient))
      ;[1 1 1] Show Popup when a Match has been found
      (EventDispatchers|BindEventtoMatchmakerMatchMatched (Variables|Default|GetNakamaRealtimeClient) (delegate Custom|MatchmakerMatched))
      ;[1 1 1] Show chat message notification
      (EventDispatchers|BindEventtoChannelMessageReceived (Variables|Default|GetNakamaRealtimeClient) (delegate Custom|OnChatMessage))
      ;[1 1 1] Display Statuses
      (EventDispatchers|BindEventtoPresenceStatusReceived (Variables|Default|GetNakamaRealtimeClient) (delegate Custom|OnStatusPresence))
      ;[1 1 1] Display simple notifications, must be sent server-side or via RPCs
      (EventDispatchers|BindEventtoNotificationReceived (Variables|Default|GetNakamaRealtimeClient) (delegate Custom|OnNotification))
      ;[1 1 1] Add Party Matchmaker Ticket (Not leader)
      (EventDispatchers|BindEventtoPartyMatchmakerTicketReceived (Variables|Default|GetNakamaRealtimeClient) (delegate Custom|OnPartyMatchmakerTicket))
      ;[1 1 1] Disconnected Event
      (EventDispatchers|BindEventtoDisconnectedEvent (Variables|Default|GetNakamaRealtimeClient) (delegate Custom|OnDisconnect))
      ;[1 1 1] Error Event
      (EventDispatchers|BindEventtoErrorEvent (Variables|Default|GetNakamaRealtimeClient) (delegate Custom|OnErrorEvent)))))

(event EventOnError
  (params (Error :type Nakama%20Error%20Structure) (Title :type Text))
  ;[1 1 1] Error Notifications
  (Default|ShowError (Variables|/Game/NakamaDemo/Widgets/WBP_Main.WBP_Main_C|GetWBP_ErrorMessage (Variables|Default|GetMainUI)) Error Title))

(event EventOnRealtimeError
  (params (RealtimeError :type Nakama%20Rt%20Error%20Structure) (Title :type Text))
  ;[1 1 1] Error Notifications
  (Default|ShowRealtimeError (Variables|/Game/NakamaDemo/Widgets/WBP_Main.WBP_Main_C|GetWBP_ErrorMessage (Variables|Default|GetMainUI)) RealtimeError Title))

(fn ConstructionScript)

(fn FindJoinedChannelbyRoomName
  (params (RoomName :type String))
  (bind _array_element (Utilities|Array|ForEachLoopwithBreak (Variables|Default|GetJoinedChannels))
    (:LoopBody
      (if (Utilities|Enum|Equal(Enum) (.RoomName (Utilities|Struct|BreakNakamaChannel _array_element)) RoomName)
        _))))